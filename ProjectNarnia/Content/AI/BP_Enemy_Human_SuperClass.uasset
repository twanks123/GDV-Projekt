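; Base Blueprint for human enemies that spawns and carries a weapon and a shield.
; On BeginPlay it spawns both at configured scales, disables their collision and attaches them to the mesh's sword and shield sockets.
; Death re-enables their collision so the player can pick them up, while destroying the enemy destroys both.
; Headshots and shield attacks set a head-hit reaction flag.
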(event Custom|DestroyWeapon
  (Actor|DestroyActor (Variables|Default|GetCurrentWeaponReference))
  (Actor|DestroyActor (Variables|Default|GetCurrentShieldReference)))

(event EventOnHeadshot
  (Variables|Default|SetReactHitHead true)
  (Development|PrintString "HEADSHOT"))

(event EventOnShieldAttack
  (Variables|Default|SetReactHitHead true))

(event EventBeginPlay
  (|CallParentFunction)
  ;[1 1 1] Equip the Weapons on Begin Play
  (CallFunction|EquipNewWeapon (Variables|Default|GetCurrentWeapon))
  (CallFunction|EquipNewShield (Variables|Default|GetCurrentShield))
  (EventDispatchers|AssignOnDestroyed (delegate Custom|DestroyWeapon)))

(event EventActorBeginOverlap
  (params (OtherActor :type Actor%20Object%20Reference)))

(event EventTick
  (params (DeltaSeconds :type Float%20%28single-precision%29))
  (|CallParentFunction 0.0))

(event EventDie
  (|CallParentFunction)
  ;[1 1 1] Enable Collision for the Weapons if this Human Enemy die, Allows Player to pick them up
  (Default|EnableCollision (Variables|Default|GetCurrentWeaponReference) false)
  (Default|EnableCollision (Variables|Default|GetCurrentShieldReference) false))

(fn ConstructionScript
  (|CallParentFunction))

(fn EquipNewWeapon
  (params (Weapon :type BP%20Weapon%20Class%20Reference))
  (bind _weaponscale (Variables|Default|GetWeaponScale))
  (bind _output_get (Variables|Default|SetCurrentWeapon Weapon))
  (bind _returnvalue (Game|SpawnActorfromClass _output_get (Math|Transform|MakeTransform "0, 0, 0" "0, 0, 0" (Math|Vector|MakeVector _weaponscale _weaponscale _weaponscale)) "Undefined" 0 0))
  (bind _output_get_2 (Variables|Default|SetCurrentWeaponReference _returnvalue))
  (Default|DisableCollision _output_get_2 false)
  (Class|Actor|AttachRootComponentto _output_get_2 (Variables|Character|GetMesh) "SwordSocket" "SnapToTarget" false) ; Attach the Weapon
  (Variables|Default|SetWeaponDrawed true))

(fn EquipNewShield
  (params (Shield :type BP%20Shield%20Class%20Reference))
  (bind _shieldscale (Variables|Default|GetShieldScale))
  (bind _output_get (Variables|Default|SetCurrentShield Shield))
  (bind _returnvalue (Game|SpawnActorfromClass _output_get (Math|Transform|MakeTransform "0, 0, 0" "0, 0, 0" (Math|Vector|MakeVector _shieldscale _shieldscale _shieldscale)) "AlwaysSpawn" 0 0))
  (bind _output_get_2 (Variables|Default|SetCurrentShieldReference _returnvalue))
  (Default|DisableCollision _output_get_2 false)
  (Class|Actor|AttachRootComponentto _output_get_2 (Variables|Character|GetMesh) "ShieldSocket" "SnapToTarget" false) ; Attach the Weapon
)