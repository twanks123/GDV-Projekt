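; Base enemy character that handles melee combat, health, death and sounds for AI enemies.
; The Behavior Tree enables attacking, Tick cancels it beyond attack range, and Attack line-traces forward to hit the player.
; Player hits feed a typed damage calculation with resistances, lifesteal and reflect, while kicks, blocks, shield, sneak and headshot events trigger heavy reactions.
; Blackboard keys receive attack range, attacker and death state.
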(event EventOnKick
  (params (Player :type Player%20Object%20Reference))
  ;[1 1 1] Called if Player kick this Enemy
  (CallFunction|ReactHeavyHit))

(event EventOnBlock
  ;[1 1 1] Called if Player blocked an Attack
  (CallFunction|ReactHeavyHit)
  (Development|PrintString "PLAyER BLOCKED MY ATTACK"))

(event EventOnShieldAttack
  ;[1 1 1] Called if Player makes an Shield Attack
  (CallFunction|ReactHeavyHit))

(event EventTick
  (params (DeltaSeconds :type Float%20%28single-precision%29))
  ;[1 1 1] Event Tick
  (|CalculateIdleTimeAndPlayAmbientSound DeltaSeconds
    (:Out
      (|CheckDistanceandDisableAttacking))))

(event EventOnHit
  (params (Player :type Player%20Object%20Reference) (HitInfo :type Hit%20Result%20Structure) (DamageMultiplier :type Float%20%28single-precision%29))
  (bind _currentweapon (Variables|/Game/Assets/Character/Player.Player_C|GetCurrentWeapon Player))
  (bind _strength (Variables|/Game/Assets/Character/Player.Player_C|GetStrength Player))
  (bind _piercedamage (Variables|/Game/Assets/Blueprints/InventorySystem/BP_Weapon.BP_Weapon_C|GetPierceDamage _currentweapon))
  (bind _bluntdmg (Variables|/Game/Assets/Blueprints/InventorySystem/BP_Weapon.BP_Weapon_C|GetBluntDmg _currentweapon))
  (bind _slashdamage (Variables|/Game/Assets/Blueprints/InventorySystem/BP_Weapon.BP_Weapon_C|GetSlashDamage _currentweapon))
  (bind _firedmg (Variables|/Game/Assets/Blueprints/InventorySystem/BP_Weapon.BP_Weapon_C|GetFireDmg _currentweapon))
  ;[1 1 1] Event On Hit (Player hit this Enemy)
  (AI|Components|Blackboard|SetValueasObject (AI|GetBlackboard self) (Utilities|Name|MakeLiteralName "Enemy") Player) ; Set the Enemy in the Blackboard
  (CallFunction|PlayRandomSound (Variables|Sounds|GetSounds_OnHit)) ; Play Sound first so Death Sound will override this
  (Development|PrintString (Utilities|String|Append "Was Hit by: " (Utilities|GetDisplayName Player) "  Target Strength: " (Utilities|String|ToString(Float) _strength) "  Pierce Damage: " (Utilities|String|ToString(Float) _piercedamage) "  Blunt Damage:  " (Utilities|String|ToString(Float) _bluntdmg) "   Slash Damage: " (Utilities|String|ToString(Float) _slashdamage) "   Fire Damage: " (Utilities|String|ToString(Float) _firedmg)) true true "(R=0.098906,G=1.000000,B=0.000000,A=1.000000)" 5.0)
  (bind (_newdealingactorhealth _newactorhealth) (CallFunction|DamageCalculation (Variables|/Game/Assets/Character/Player.Player_C|GetPlayerCurrentHealth Player) (Variables|Default|GetCurrent%20Health) (* _piercedamage DamageMultiplier) (* _bluntdmg DamageMultiplier) (* _slashdamage DamageMultiplier) (* _firedmg DamageMultiplier) (Variables|Resistances|GetPierceRes) (Variables|Resistances|GetBluntRes) (Variables|Resistances|GetSlashRes) (Variables|Resistances|GetFireRes) (Variables|/Game/Assets/Blueprints/InventorySystem/BP_Weapon.BP_Weapon_C|GetLifesteal _currentweapon) (Variables|Resistances|GetDmgReflect) _strength))
  (Default|SetHealth Player _newdealingactorhealth)
  (CallFunction|SetEnemyHealth _newactorhealth))

(event EventOnSneakAttack
  ;[1 1 1] Called if Player made an Sneak Attack
  (CallFunction|ReactHeavyHit))

(event EventOnHeadshot
  ;[1 1 1] Called if Player made an Headshot
  (CallFunction|DecreaseHealth (Variables|Default|GetExtraDamageHeadshot))
  (CallFunction|ReactHeavyHit)
  (Development|PrintString "HEADSHOT" true true "(R=1.000000,G=0.000000,B=0.092125,A=1.000000)" 5.0))

(event EventSetAttackingtoTrue
  ;[1 1 1] Called from Behaviour Tree - Enable Attacking
  (bind _asplayer (Utilities|Casting|CastToPlayer (Game|Player|GetPlayerPawn 0)))
  (if (Variables|/Game/Assets/Character/Player.Player_C|GetisDeath _asplayer)
    (Variables|BoolVariables|SetisAttacking false)
    (else
      (Variables|BoolVariables|SetisAttacking true)
      (CallFunction|RotateTowardsPlayer)
      (if (Variables|Default|GetDontMoveOnAttack)
        (CallFunction|SetMovement false)))))

(event EventBeginPlay
  (bind _self self)
  (bind _returnvalue (AI|GetBlackboard _self))
  ;[1 1 1] Event Begin Play
  (Variables|Default|SetCurrent%20Health (Variables|Default|GetMax%20Health))
  (Variables|/Script/Engine.CharacterMovementComponent|SetMaxWalkSpeed (Variables|Character|GetCharacterMovement) (Variables|Default|GetMovementSpeed))
  (AI|Components|Blackboard|SetValueasFloat _returnvalue (Utilities|Name|MakeLiteralName "AttackRange") (Variables|Default|GetAttackRange)) ; Set the Attack Range in the Blackboard
  (AI|Components|Blackboard|SetValueasFloat _returnvalue (Utilities|Name|MakeLiteralName "DistanceToEnemy") 9999.0) ; Distance is set to 0 default, thats why i set it here to 9999
)

(fn ConstructionScript)

(fn Die
  (Variables|BoolVariables|SetIsDead true)
  (Collision|SetActorEnableCollision false)
  (CallFunction|PlayRandomSound (Variables|Sounds|GetSounds_OnDeath))
  (AI|Components|Blackboard|SetValueasBool (AI|GetBlackboard self) (Utilities|Name|MakeLiteralName "IsDead") true))

(fn Attack
  (params (DamageMultiplier :type Float%20%28single-precision%29))
  (CallFunction|PlayRandomSound (Variables|Sounds|GetSounds_OnAttack))
  (bind (_player _hit_result) (Utilities|TraceforPlayer)
    (:Ray%20hit%20Player
      (Default|OnHit _player self _hit_result DamageMultiplier))))

(fn RotateTowardsPlayer
  (Transformation|SetActorRotation (Math|Rotator|MakeRotator 0.0 0.0 (.yaw (Math|Rotator|FindLookatRotation (Transformation|GetActorLocation) (Transformation|GetActorLocation (Game|Player|GetPlayerPawn 0)))))))

(fn SetMovement
  (params (Can%20Move :type Boolean))
  (bind _charactermovement (Variables|Character|GetCharacterMovement))
  (if Can%20Move
    (Variables|/Script/Engine.CharacterMovementComponent|SetMaxWalkSpeed _charactermovement (Variables|Default|GetMovementSpeed))
    (else
      (Variables|/Script/Engine.CharacterMovementComponent|SetMaxWalkSpeed _charactermovement 0.0))))

(fn PlaySound
  (params (Sound :type Sound%20Cue%20Object%20Reference))
  (bind _audiocomponent (Variables|Default|GetAudioComponent))
  (Utilities|IsValid Sound
    (:Is%20Valid
      (Audio|Components|Audio|SetSound _audiocomponent Sound)
      (Audio|Components|Audio|Play _audiocomponent 0.0))))

(fn DecreaseHealth
  (params (Damage :type Float%20%28single-precision%29))
  (bind _output_get (Variables|Default|SetCurrent%20Health (Math|Float|Max(Float) (- (Variables|Default|GetCurrent%20Health) Damage) 0.0)))
  (Development|PrintString (Utilities|String|ToString(Float) _output_get))
  (if (<= _output_get 0.0)
    (CallFunction|Die))
  (return (Variables|Default|GetCurrent%20Health)))

(fn PlayRandomSound
  (params (Sound%20Array :type Array%20of%20Sound%20Cue%20Object%20References))
  (CallFunction|PlaySound (Utilities|Array|Get(acopy) Sound%20Array (Math|Random|RandomInteger (Utilities|Array|Length Sound%20Array)))))

(fn ReactHeavyHit
  (Variables|BoolVariables|SetReactHit true)
  (CallFunction|PlayRandomSound (Variables|Sounds|GetSounds_OnHit)))

(fn SetEnemyHealth
  (params (NewEnemyHealth :type Float%20%28single-precision%29))
  (bind _output_get (Variables|Default|SetCurrent%20Health (Math|Float|Clamp(Float) NewEnemyHealth 0.0 (Variables|Default|GetMax%20Health))))
  (Development|PrintString (Utilities|String|Append "I'm " (Utilities|GetDisplayName self) " and my new Health is: " (Utilities|String|ToString(Float) (Variables|Default|GetCurrent%20Health))))
  (if (<= _output_get 0.0)
    (CallFunction|Die)))