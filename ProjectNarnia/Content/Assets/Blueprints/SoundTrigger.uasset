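; SoundTrigger is a trigger actor that plays a one-shot 2D sound the first time the Player overlaps it.
; It finds the MusicMaster on BeginPlay, ducks its volume while the sound plays, then restores it after the sound's duration.
; DoOnce gates keep it from replaying, and an invalid sound prints a debug message naming the trigger.
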(event EventBeginPlay
  (bind _outactors (Actor|GetAllActorsOfClass "/Game/Assets/Blueprints/MusicMaster.MusicMaster_C"))
  (Variables|Default|SetMusicManager (Utilities|Array|Get(acopy) _outactors)))

(event EventActorBeginOverlap
  (params (OtherActor :type Actor%20Object%20Reference))
  (bind _sound (Variables|Default|GetSound))
  (bind _musicmanager (Variables|Default|GetMusicManager))
  (Utilities|Casting|CastToPlayer OtherActor)
  (Utilities|FlowControl|DoOnce false
    (:Completed
      (Utilities|IsValid _sound
        (:Is%20Valid
          (Utilities|FlowControl|DoOnce false
            (:Completed
              (Audio|PlaySound2D _sound (Variables|Default|GetVolumeMultiplier))
              (Default|SetVolume _musicmanager 0.35)
              (Utilities|FlowControl|Delay (Variables|/Script/Engine.SoundBase|GetDuration (Variables|Default|GetSound)))
              (Default|SetVolume _musicmanager 1.0))))
        (:Is%20Not%20Valid
          (Development|PrintString (Utilities|String|Append "Sound in TriggerBox " (Utilities|GetDisplayName self) " is not valid!")))))))

(fn ConstructionScript)