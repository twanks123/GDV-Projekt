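; Music manager that plays the game's soundtrack cues, such as the castle entrance and Battle of the Five Armies, through one audio component.
; PlayMusic sets the track and start time, and Tick accumulates elapsed time so ContinueMusic can fade back in where StopMusic faded out.
; The audio-finished event chains the castle entrance tracks into the after-castle music.
; SetVolume adjusts the multiplier, which Tick also prints every frame.
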(event Custom|OnAudioFinished
  (bind _audio (Variables|Default|GetAudio))
  (bind _sound (Variables|/Script/Engine.AudioComponent|GetSound _audio))
  (if (== _sound (Variables|Default|GetCastleEntranceMusic))
    (CallFunction|PlayMusic (Variables|Default|GetCastleEntranceMusic_2) 0.0)
    (elif (== _sound (Variables|Default|GetCastleEntranceMusic_2))
      (CallFunction|PlayMusic (Variables|Default|GetMusicAfterCastleMusic) 0.0))))

(event EventTick
  (params (DeltaSeconds :type Float%20%28single-precision%29))
  (Development|PrintString (Utilities|String|ToString(Float) (Variables|/Script/Engine.AudioComponent|GetVolumeMultiplier (Variables|Default|GetAudio))))
  (if (Variables|Default|GetIsPlayingMusic)
    (Variables|Default|SetTime (+ (Variables|Default|GetTime) DeltaSeconds))))

(event EventBeginPlay
  (EventDispatchers|BindEventtoOnAudioFinished (Variables|Default|GetAudio) (delegate Custom|OnAudioFinished)))

(fn ConstructionScript)

(fn PlayBattleOftheFiveArmies
  (CallFunction|PlayMusic (Variables|Default|GetHobbitbattleofthearmies) (Variables|Default|GetStartTimeBattleOfTheFiveArmies)))

(fn StopMusic
  (Audio|Components|Audio|FadeOut (Variables|Default|GetAudio) 2.0 0.0 :!class /Script/Engine.AudioComponent)
  (Variables|Default|SetIsPlayingMusic false))

(fn ContinueMusic
  (Audio|Components|Audio|FadeIn (Variables|Default|GetAudio) 2.0 1.0 (Variables|Default|GetTime) :!class /Script/Engine.AudioComponent)
  (Variables|Default|SetIsPlayingMusic true))

(fn PlayCastleEntranceMusic
  (CallFunction|PlayMusic (Variables|Default|GetCastleEntranceMusic) 0.0))

(fn PlayMusic
  (params (Music :type Sound%20Cue%20Object%20Reference) (StartTime :type Float%20%28single-precision%29))
  (bind _audio (Variables|Default|GetAudio))
  (Audio|Components|Audio|SetSound _audio Music)
  (Audio|Components|Audio|Play _audio StartTime)
  (Variables|Default|SetIsPlayingMusic true)
  (Variables|Default|SetTime StartTime))

(fn SetVolume
  (params (Volume :type Float%20%28single-precision%29))
  (bind _audio (Variables|Default|GetAudio))
  (Utilities|IsValid (Variables|/Script/Engine.AudioComponent|GetSound _audio)
    (:Is%20Valid
      (Audio|Components|Audio|SetVolumeMultiplier _audio Volume :!class /Script/Engine.AudioComponent))))