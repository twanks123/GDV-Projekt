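; Fire effect actor that sets the player on fire while inside its trigger volume and clears that state when they leave.
; Trigger overlap events cast to the Player and toggle its on-fire flag.
; SetActive switches the fire audio, particle effect and trigger collision together, and BeginPlay applies the configured Active state through it.
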(event OnComponentBeginOverlap(Trigger)
  (params (OtherActor :type Actor%20Object%20Reference) (OtherComp :type Primitive%20Component%20Object%20Reference) (OtherBodyIndex :type Integer) (bFromSweep :type Boolean) (SweepResult :type Hit%20Result%20Structure%20%28by%20ref%29))
  ;[1 1 1] Set the Player on Fire
  (bind _asplayer (Utilities|Casting|CastToPlayer OtherActor))
  (Default|SetIsonFire _asplayer true))

(event OnComponentEndOverlap(Trigger)
  (params (OtherActor :type Actor%20Object%20Reference) (OtherComp :type Primitive%20Component%20Object%20Reference) (OtherBodyIndex :type Integer))
  ;[1 1 1] Deactivate Fire at the Player
  (bind _asplayer (Utilities|Casting|CastToPlayer OtherActor))
  (Default|SetIsonFire _asplayer false))

(event EventBeginPlay
  (CallFunction|SetActive (Variables|Default|GetActive)))

(fn ConstructionScript)

(fn SetActive
  (params (Active :type Boolean))
  (bind _trigger (Variables|Default|GetTrigger))
  (Variables|Default|SetActive Active)
  (Components|Activation|SetActive (Variables|Audio|GetFire%20Audio) (Variables|Default|GetActive) false)
  (Components|Activation|SetActive (Variables|Default|GetP_Fire) (Variables|Default|GetActive) false)
  (if (Variables|Default|GetActive)
    (Collision|SetCollisionEnabled _trigger "QueryAndPhysics")
    (else
      (Collision|SetCollisionEnabled _trigger "NoCollision"))))