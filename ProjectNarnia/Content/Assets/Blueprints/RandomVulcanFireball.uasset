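; Vulcano fireball actor that periodically erupts a particle effect with sound at a fixed time interval.
; Tick accumulates elapsed time and, once it reaches TimeBetweenFireballs, resets it, gives the ParticleSystem a random yaw, reactivates it and plays the Audio component.
; The construction script assigns the configurable SoundWhenFireball to the audio component.
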(event EventTick
  (params (DeltaSeconds :type Float%20%28single-precision%29))
  (bind _output_get (Variables|Default|SetPassedTime (+ DeltaSeconds (Variables|Default|GetPassedTime))))
  (if (>= _output_get (Variables|Default|GetTimeBetweenFireballs))
    (Variables|Default|SetPassedTime 0.0)
    (Transformation|SetRelativeRotation (Variables|Default|GetParticleSystem) (Math|Rotator|MakeRotator 0.0 0.0 (Math|Conversions|ToFloat(Integer) (Math|Random|RandomInteger 180))) false false)
    (Components|Activation|Activate (Variables|Default|GetParticleSystem) true)
    (Audio|Components|Audio|Play (Variables|Default|GetAudio) 0.0)))

(fn ConstructionScript
  (Audio|Components|Audio|SetSound (Variables|Default|GetAudio) (Variables|Default|GetSoundWhenFireball)))