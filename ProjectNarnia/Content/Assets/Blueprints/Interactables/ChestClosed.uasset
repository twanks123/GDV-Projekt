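; Locked chest interactable that opens when the player has the item named by KeyName.
; On interaction it tries to remove that item from the Player's inventory; success sets ChestIsOpen, plays the open sound and swaps the mesh to the open version.
; Failure plays the closed sound if the chest is shut and the cue is idle.
; Key removal runs before any open-state check, so an open chest can consume another key.
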(event EventOnInteract
  (params (Actor :type Actor%20Object%20Reference))
  (bind _chest_cue (Variables|Default|GetChest%20Cue))
  (bind _chest_cue_2 (Variables|Default|GetChest%20Cue))
  (bind _asplayer (Utilities|Casting|CastToPlayer Actor))
  (bind _itemsuccessfullyremoved (Default|RemoveInventoryItembyName _asplayer (Variables|Default|GetKeyName)))
  (if _itemsuccessfullyremoved
    (Variables|Default|SetChestIsOpen true)
    (Audio|Components|Audio|SetSound _chest_cue_2 (Variables|Default|GetSoundChestIsOpen))
    (Audio|Components|Audio|Play _chest_cue_2 0.0)
    (Components|StaticMesh|SetStaticMesh (Variables|Default|GetSM_Item) (Variables|Default|GetChestOpen))
    (elif (not (Variables|Default|GetChestIsOpen))
      ;[1 1 1] Play a Sound if Player wants to open the Door but is closed
      (if (not (Components|Activation|IsActive _chest_cue))
        (Audio|Components|Audio|SetSound _chest_cue (Variables|Default|GetSoundChestIsClosed))
        (Audio|Components|Audio|Play _chest_cue 0.0)))))

(fn ConstructionScript
  (|CallParentFunction))