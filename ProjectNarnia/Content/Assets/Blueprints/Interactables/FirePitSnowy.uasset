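; Interactable fire pit that the player can light or put out, restoring player health while it burns.
; Interacting toggles the particles, audio and point light, and starts or stops a timeline that feeds health regeneration, scaled by rate and frame time.
; Sphere overlap also starts the timeline when lit and stops it on exit, with a debug print.
; ActiveOnStart sets initial particle and audio state at construction and BeginPlay.
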(event OnComponentBeginOverlap(Sphere)
  (params (OtherActor :type Actor%20Object%20Reference) (OtherComp :type Primitive%20Component%20Object%20Reference) (OtherBodyIndex :type Integer) (bFromSweep :type Boolean) (SweepResult :type Hit%20Result%20Structure%20%28by%20ref%29))
  ;[1 1 1] Player Health-Regeneration
  (if (Components|Activation|IsActive (Variables|Default|GetParticleSystem))
    (bind _asplayer (Utilities|Casting|CastToPlayer OtherActor))
    (Variables|Default|SetPlayer _asplayer)
    (bind _healthregeneration (Timeline|Timeline_0 Play)
      (:Update
        (Default|IncreaseHealth (Variables|Default|GetPlayer) (* _healthregeneration (Variables|Default|GetRegenerationPerSecond) (Utilities|Time|GetWorldDeltaSeconds)))))))

(event OnComponentEndOverlap(Sphere)
  (params (OtherActor :type Actor%20Object%20Reference) (OtherComp :type Primitive%20Component%20Object%20Reference) (OtherBodyIndex :type Integer))
  ;[1 1 1] Player Health-Regeneration
  (Utilities|Casting|CastToPlayer OtherActor)
  (Development|PrintString "Hello")
  (bind _healthregeneration (Timeline|Timeline_0 Stop)
    (:Update
      (Default|IncreaseHealth (Variables|Default|GetPlayer) (* _healthregeneration (Variables|Default|GetRegenerationPerSecond) (Utilities|Time|GetWorldDeltaSeconds))))))

(event EventOnInteract
  (params (Actor :type Actor%20Object%20Reference))
  (bind _pointlight (Variables|Default|GetPointLight))
  (bind _particlesystem (Variables|Default|GetParticleSystem))
  ;[1 1 1] On Interact
  (if (Components|Activation|IsActive _particlesystem)
    (Components|Activation|SetActive _particlesystem false false)
    (Rendering|Components|Light|SetIntensity _pointlight 0.0)
    ;[1 1 1] Player Health-Regeneration
    (bind _healthregeneration (Timeline|Timeline_0 Stop)
      (:Update
        (Default|IncreaseHealth (Variables|Default|GetPlayer) (* _healthregeneration (Variables|Default|GetRegenerationPerSecond) (Utilities|Time|GetWorldDeltaSeconds)))))
    (else
      (Components|Activation|SetActive _particlesystem true false)
      (Rendering|Components|Light|SetIntensity _pointlight 5e+01)
      (Timeline|Timeline_0 Play))))

(event EventBeginPlay
  (bind _audio_0 (Variables|Default|GetAudio_0))
  ;[1 1 1] Get the Player
  (bind _asplayer (Utilities|Casting|CastToPlayer (Game|Player|GetPlayerPawn 0)))
  (Variables|Default|SetPlayer _asplayer)
  (if (Variables|Default|GetActiveOnStart)
    (Components|Activation|SetActive _audio_0 true false)
    (else
      (Components|Activation|SetActive _audio_0 false false))))

(fn ConstructionScript
  (|CallParentFunction)
  (if (Variables|Default|GetActiveOnStart)
    (Components|Activation|SetActive (Variables|Default|GetAudio_0) true false)
    (else
      (Components|Activation|SetActive (Variables|Default|GetParticleSystem) false false))))