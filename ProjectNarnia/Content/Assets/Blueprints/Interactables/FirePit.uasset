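; FirePit is an interactable fire pit that toggles its fire and heals a nearby player while lit.
; Interacting switches the particles, audio and point light on or off and plays or stops the RegenerateHealth timeline.
; Sphere overlap caches the player and starts the timeline if lit, and end overlap stops it.
; Each timeline update increases player health by its curve value, RegenerationPerSecond and delta time.
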(event OnComponentBeginOverlap(Sphere)
  (params (OtherActor :type Actor%20Object%20Reference) (OtherComp :type Primitive%20Component%20Object%20Reference) (OtherBodyIndex :type Integer) (bFromSweep :type Boolean) (SweepResult :type Hit%20Result%20Structure%20%28by%20ref%29))
  ;[1 1 1] Player Health-Regeneration
  (bind _asplayer (Utilities|Casting|CastToPlayer OtherActor))
  (Variables|Default|SetPlayer _asplayer)
  (if (Components|Activation|IsActive (Variables|Default|GetParticleSystem))
    (bind _healthregeneration (Timeline|RegenerateHealth Play)
      (:Update
        (Default|IncreaseHealth (Variables|Default|GetPlayer) (* _healthregeneration (Variables|Default|GetRegenerationPerSecond) (Utilities|Time|GetWorldDeltaSeconds)))))))

(event OnComponentEndOverlap(Sphere)
  (params (OtherActor :type Actor%20Object%20Reference) (OtherComp :type Primitive%20Component%20Object%20Reference) (OtherBodyIndex :type Integer))
  ;[1 1 1] Player Health-Regeneration
  (Utilities|Casting|CastToPlayer OtherActor)
  (bind _healthregeneration (Timeline|RegenerateHealth Stop)
    (:Update
      (Default|IncreaseHealth (Variables|Default|GetPlayer) (* _healthregeneration (Variables|Default|GetRegenerationPerSecond) (Utilities|Time|GetWorldDeltaSeconds))))))

(event EventOnInteract
  (params (Actor :type Actor%20Object%20Reference))
  (bind _pointlight (Variables|Default|GetPointLight))
  (bind _particlesystem (Variables|Default|GetParticleSystem))
  ;[1 1 1] On Interact
  (if (Components|Activation|IsActive _particlesystem)
    (Components|Activation|SetActive _particlesystem false false)
    (Rendering|Components|Light|SetIntensity _pointlight 0.0)
    ;[1 1 1] Player Health-Regeneration
    (bind _healthregeneration (Timeline|RegenerateHealth Stop)
      (:Update
        (Default|IncreaseHealth (Variables|Default|GetPlayer) (* _healthregeneration (Variables|Default|GetRegenerationPerSecond) (Utilities|Time|GetWorldDeltaSeconds)))))
    (else
      (Components|Activation|SetActive _particlesystem true false)
      (Rendering|Components|Light|SetIntensity _pointlight 2e+01)
      (Timeline|RegenerateHealth Play))))

(fn ConstructionScript
  (|CallParentFunction))