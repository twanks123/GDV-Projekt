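; BP_Door is an interactable door that swings open based on the side the interacting actor comes from and closes on the next interaction.
; A FlipFlop on OnInteract alternates opening and closing.
; Opening unrotates the door-to-actor offset and uses its Y sign to pick one of two timelines driving SMItem's relative yaw.
; Closing reverses the timeline matching the sign of the current yaw.
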(event EventBeginPlay)

(event EventActorBeginOverlap
  (params (OtherActor :type Actor%20Object%20Reference)))

(event EventTick
  (params (DeltaSeconds :type Float%20%28single-precision%29)))

(event EventOnInteract
  (params (Actor :type Actor%20Object%20Reference))
  (bind _sm_item (Variables|Default|GetSM_Item))
  ;[1 1 1] Open the Door on Interact based on which Direction the other Actor is coming from
  (Utilities|FlowControl|FlipFlop
    (:A
      (if (> (.y (Math|Vector|UnrotateVector (- (Transformation|GetActorLocation) (Transformation|GetActorLocation Actor)) (Transformation|GetActorRotation))) 0.0) ; Open the Door
        (bind _doorrotation (Timeline|DoorMovement Play)
          (:Update
            (Transformation|SetRelativeRotation _sm_item (Math|Rotator|MakeRotator 0.0 0.0 _doorrotation) false false)))
        (else
          (bind _doorrotation_2 (Timeline|DoorMovementOtherDirection Play)
            (:Update
              (Transformation|SetRelativeRotation _sm_item (Math|Rotator|MakeRotator 0.0 0.0 _doorrotation_2) false false))))))
    (:B
      (if (< (.yaw (Variables|/Script/Engine.SceneComponent|GetRelativeRotation (Variables|Default|GetSM_Item))) 0.0) ; Close the Door
        (Timeline|DoorMovement Reverse)
        (else
          (Timeline|DoorMovementOtherDirection Reverse))))))

(fn ConstructionScript)