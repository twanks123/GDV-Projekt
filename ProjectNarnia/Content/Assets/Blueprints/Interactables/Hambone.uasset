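; Hambone is an interactable health pickup that heals the player who uses it.
; On interact it runs the parent logic, increases the interacting Player's health by its Health value and destroys itself, doing nothing further for non-player actors.
; On BeginPlay it builds its ItemInfo text from that Health value.
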(event EventOnInteract
  (params (Actor :type Actor%20Object%20Reference))
  (|CallParentFunction Actor)
  (bind _asplayer (Utilities|Casting|CastToPlayer Actor))
  (Default|IncreaseHealth _asplayer (Variables|Default|GetHealth))
  (Actor|DestroyActor))

(event EventBeginPlay
  (Variables|Default|SetItemInfo (Utilities|String|Append "Restore's " (Utilities|String|ToString(Float) (Variables|Default|GetHealth)) " Health.")))

(fn ConstructionScript
  (|CallParentFunction))