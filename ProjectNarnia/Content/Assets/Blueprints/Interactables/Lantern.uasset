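; Lantern is an equippable item that gives off a flickering point light while equipped.
; The construction script applies the configured intensity, color and temperature, and BeginPlay caches that intensity as the flicker baseline.
; Equipping disables actor collision, shows the mesh and plays a timeline that sets brightness to its curve times the baseline, raised to FlickeringStrength.
; Unequipping zeroes the light, hides the mesh and stops the timeline.
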(event EventBeginPlay
  (|CallParentFunction)
  (Variables|Default|SetInitialLightIntensity (Variables|/Script/Engine.LightComponentBase|GetIntensity (Variables|Default|GetPointLight))))

(event EventOnEquip
  (|CallParentFunction)
  (Collision|SetActorEnableCollision false)
  (Rendering|Components|Light|SetIntensity (Variables|Default|GetPointLight) 5e+03)
  (Development|SetHiddeninGame (Variables|Default|GetSM_Item) false false)
  ;[1 1 1] Light Flickering based on a Timeline
  (bind _lightintensity (Timeline|Timeline_0 Play)
    (:Update
      (Rendering|Components|Light|SetIntensity (Variables|Default|GetPointLight) (Math|Float|Power (* _lightintensity (Variables|Default|GetInitialLightIntensity)) (Variables|Default|GetFlickeringStrength))))))

(event EventOnUnequip
  (|CallParentFunction)
  (Rendering|Components|Light|SetIntensity (Variables|Default|GetPointLight) 0.0)
  (Development|SetHiddeninGame (Variables|Default|GetSM_Item) true false)
  ;[1 1 1] Light Flickering based on a Timeline
  (bind _lightintensity (Timeline|Timeline_0 Stop)
    (:Update
      (Rendering|Components|Light|SetIntensity (Variables|Default|GetPointLight) (Math|Float|Power (* _lightintensity (Variables|Default|GetInitialLightIntensity)) (Variables|Default|GetFlickeringStrength))))))

(fn ConstructionScript
  (bind _pointlight (Variables|Default|GetPointLight))
  (|CallParentFunction)
  (Rendering|Components|Light|SetIntensity _pointlight (Variables|Default|GetIntensity))
  (Rendering|Components|Light|SetLightColor _pointlight (Variables|Default|GetLightColor) true)
  (Class|LightComponent|SetTemperature _pointlight (Variables|Default|GetTemperature)))