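; Fort brazier Blueprint with a point light and flicker logic for its fire.
; The construction script applies an exposed attenuation radius to the light, and BeginPlay caches its starting intensity.
; A timeline's update sets intensity to its curve value times that baseline, raised to a flickering-strength exponent.
; No event in the graph starts this timeline.
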(event EventBeginPlay
  ;[1 1 1] Set Initial Light Intensity for this Fire when Game starts
  (Variables|Default|SetInitialLightIntensity (Variables|/Script/Engine.LightComponentBase|GetIntensity (Variables|Default|GetPointLight))))

(fn ConstructionScript
  (Rendering|Lighting|SetAttenuationRadius (Variables|Default|GetPointLight) (Variables|Default|GetAttenuationRadius)))