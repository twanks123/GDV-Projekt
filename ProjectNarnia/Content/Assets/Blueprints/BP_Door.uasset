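; BP_Door is a swinging door Blueprint that opens away from whichever side an actor enters its trigger box, then closes when an overlap ends.
; On overlap, it unrotates the offset to the actor by the door's rotation and uses the sign of local Y to play one of two timelines driving Door's relative yaw.
; On end overlap, the sign of the current yaw selects which timeline to reverse.
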(event OnComponentBeginOverlap(Box)
  (params (OtherActor :type Actor%20Object%20Reference) (OtherComp :type Primitive%20Component%20Object%20Reference) (OtherBodyIndex :type Integer) (bFromSweep :type Boolean) (SweepResult :type Hit%20Result%20Structure%20%28by%20ref%29))
  (bind _door (Variables|Default|GetDoor))
  ;[1 1 1] Open the Door based on which Direction the other Actor is coming from
  (if (> (.y (Math|Vector|UnrotateVector (- (Transformation|GetActorLocation) (Transformation|GetActorLocation OtherActor)) (Transformation|GetActorRotation))) 0.0)
    (bind _doorrotation (Timeline|DoorMovement Play)
      (:Update
        (Transformation|SetRelativeRotation _door (Math|Rotator|MakeRotator 0.0 0.0 _doorrotation) false false)))
    (else
      (bind _doorrotation_2 (Timeline|DoorMovementOtherDirection Play)
        (:Update
          (Transformation|SetRelativeRotation _door (Math|Rotator|MakeRotator 0.0 0.0 _doorrotation_2) false false))))))

(event OnComponentEndOverlap(Box)
  (params (OtherActor :type Actor%20Object%20Reference) (OtherComp :type Primitive%20Component%20Object%20Reference) (OtherBodyIndex :type Integer))
  (bind _door (Variables|Default|GetDoor))
  ;[1 1 1] Open the Door based on which Direction the other Actor is coming from
  (if (< (.yaw (Variables|/Script/Engine.SceneComponent|GetRelativeRotation (Variables|Default|GetDoor))) 0.0)
    (bind _doorrotation (Timeline|DoorMovement Reverse)
      (:Update
        (Transformation|SetRelativeRotation _door (Math|Rotator|MakeRotator 0.0 0.0 _doorrotation) false false)))
    (else
      (bind _doorrotation_2 (Timeline|DoorMovementOtherDirection Reverse)
        (:Update
          (Transformation|SetRelativeRotation _door (Math|Rotator|MakeRotator 0.0 0.0 _doorrotation_2) false false))))))

(event EventBeginPlay)

(event EventActorBeginOverlap
  (params (OtherActor :type Actor%20Object%20Reference)))

(event EventTick
  (params (DeltaSeconds :type Float%20%28single-precision%29)))

(fn ConstructionScript)