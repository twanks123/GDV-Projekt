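; Torch Blueprint with a point light whose color and intensity are set from variables in the Construction Script.
; BeginPlay stores the light's starting intensity as the base for a flicker effect.
; A LightFlicker timeline is meant to scale that intensity, raised to a FlickeringStrength exponent, and move the light for realism.
; Both the flicker and movement logic are unconnected and never run, so the light stays static.
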(event EventBeginPlay
  ;[1 1 1] Set Initial Light Intensity for this Torch when Game starts
  (Variables|Default|SetInitialLightIntensity (Variables|/Script/Engine.LightComponentBase|GetIntensity (Variables|Default|GetPointLight))))

(fn ConstructionScript
  (bind _pointlight (Variables|Default|GetPointLight))
  (Rendering|Components|Light|SetLightColor _pointlight (Variables|Light|GetLightColor) true)
  (Rendering|Components|Light|SetIntensity _pointlight (Variables|Light|GetLightIntensity)))