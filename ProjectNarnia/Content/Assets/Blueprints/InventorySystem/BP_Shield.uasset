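; BP_Shield is a shield item in the inventory system that can toggle its mesh collision and physics.
; On BeginPlay it runs the parent logic and caches the SMItem component's relative transform.
; EnableCollision turns on query and physics collision with optional simulation.
; DisableCollision switches both off and can restore the cached transform, undoing any displacement from physics.
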(event EventBeginPlay
  (|CallParentFunction)
  (Variables|Default|SetDefaultTransform (Transformation|GetRelativeTransform (Variables|Default|GetSM_Item))))

(event EventActorBeginOverlap
  (params (OtherActor :type Actor%20Object%20Reference)))

(event EventTick
  (params (DeltaSeconds :type Float%20%28single-precision%29)))

(fn ConstructionScript
  (|CallParentFunction))

(fn EnableCollision
  (params (SimulatePhysics :type Boolean))
  (bind _sm_item (Variables|Default|GetSM_Item))
  (Physics|SetSimulatePhysics _sm_item SimulatePhysics)
  (Collision|SetCollisionEnabled _sm_item "QueryAndPhysics"))

(fn DisableCollision
  (params (Reset%20Transform :type Boolean))
  (bind _sm_item (Variables|Default|GetSM_Item))
  (Physics|SetSimulatePhysics _sm_item false)
  (Collision|SetCollisionEnabled _sm_item "NoCollision")
  (if Reset%20Transform
    (Transformation|SetRelativeTransform _sm_item (Variables|Default|GetDefaultTransform) false false)))