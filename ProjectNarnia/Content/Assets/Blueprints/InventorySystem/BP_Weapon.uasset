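; BP_Weapon is a weapon actor in the inventory system that toggles its item mesh between a physics-simulated state and an inert one.
; It caches the relative transform of SMItem at BeginPlay.
; EnableCollision turns on physics and collision, while DisableCollision turns both off and restores the cached transform, undoing any offset the mesh gained while simulating.
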(event EventBeginPlay
  (Variables|Default|SetDefaultTransform (Transformation|GetRelativeTransform (Variables|Default|GetSM_Item))))

(event EventActorBeginOverlap
  (params (OtherActor :type Actor%20Object%20Reference)))

(event EventTick
  (params (DeltaSeconds :type Float%20%28single-precision%29)))

(fn ConstructionScript
  (|CallParentFunction))

(fn DisableCollision
  (bind _sm_item (Variables|Default|GetSM_Item))
  (Physics|SetSimulatePhysics _sm_item false)
  (Collision|SetCollisionEnabled _sm_item "NoCollision")
  (Transformation|SetRelativeTransform _sm_item (Variables|Default|GetDefaultTransform) false false))

(fn EnableCollision
  (bind _sm_item (Variables|Default|GetSM_Item))
  (Physics|SetSimulatePhysics _sm_item true)
  (Collision|SetCollisionEnabled _sm_item "QueryAndPhysics"))