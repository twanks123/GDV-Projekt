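; BP_Equipment is an inventory system actor for an equippable item that tracks whether it is equipped.
; OnEquip and OnUnequip set the IsEquipped flag and print the item's display name with a status message.
; It has no other gameplay logic, as the event graph holds only disabled placeholder events and the construction script just calls its parent.
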(event EventBeginPlay
  (|CallParentFunction))

(event EventActorBeginOverlap
  (params (OtherActor :type Actor%20Object%20Reference)))

(event EventTick
  (params (DeltaSeconds :type Float%20%28single-precision%29)))

(fn ConstructionScript
  (|CallParentFunction))

(fn OnEquip
  (Variables|Default|SetisEquipped true)
  (Development|PrintString (Utilities|String|Append (Utilities|GetDisplayName self) " was equipped!")))

(fn OnUnequip
  (Variables|Default|SetisEquipped false)
  (Development|PrintString (Utilities|String|Append (Utilities|GetDisplayName self) " were unequipped!")))