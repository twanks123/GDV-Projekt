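; BP_SwingingChandelier is a chandelier actor meant to sway back and forth.
; BeginPlay uses SwingOtherDirection to choose the axis, storing two small opposing rotations.
; The SwayAnimation timeline's update lerps the static mesh's world rotation between them.
; No wire in the graph starts that timeline, so any motion would depend on an autoplay setting not shown here.
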(event EventBeginPlay
  (if (Variables|Default|GetSwingOtherDirection)
    (Variables|Default|SetRotation1 "0, 0,5.000000")
    (Variables|Default|SetRotation2 "0, 0,-5.000000")
    (else
      (Variables|Default|SetRotation1 "5.000000, 0,0.000000")
      (Variables|Default|SetRotation2 "-5.000000, 0,0.000000"))))

(event EventActorBeginOverlap
  (params (OtherActor :type Actor%20Object%20Reference)))

(fn ConstructionScript)